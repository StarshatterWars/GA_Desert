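; HealthPickup is a pickup actor that restores a chunk of the player's health on overlap.
; It checks that the overlapping actor's class is exactly MyCharacter, then applies the heal to player 0's character rather than the overlapping actor.
; Healing happens only below full health and is clamped to the maximum, after which the pickup plays a sound and destroys itself.
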(event OnComponentBeginOverlap()
  (params (OtherActor :type Actor%20Object%20Reference) (OtherComp :type Primitive%20Component%20Object%20Reference) (OtherBodyIndex :type Integer) (bFromSweep :type Boolean) (SweepResult :type Hit%20Result%20Structure%20%28by%20ref%29))
  (if (== (Utilities|GetClass OtherActor) "/Game/Blueprints/MyCharacter.MyCharacter_C")
    (bind _asmycharacter_c (Utilities|Casting|CastToMyCharacter (Game|GetPlayerCharacter 0)))
    (if (< (Variables|/Game/Blueprints/MyCharacter.MyCharacter_C|GetPlayerHealth _asmycharacter_c) 1e+02)
      (Variables|/Game/Blueprints/MyCharacter.MyCharacter_C|SetPlayerHealth _asmycharacter_c (Math|Float|Min(Float) (+ (Variables|/Game/Blueprints/MyCharacter.MyCharacter_C|GetPlayerHealth _asmycharacter_c) 5e+01) 1e+02))
      (Class|GameplayStatics|PlaySoundAttached "/Engine/EditorSounds/Notifications/CompileSuccess.CompileSuccess" (VehicleSound|GetRootComponent))
      (Actor|DestroyActor))))

(fn ConstructionScript)