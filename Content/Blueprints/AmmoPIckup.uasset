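; AmmoPIckup is a pickup actor that refills the player's ammo.
; When its Box1 component begins overlapping an actor whose class is exactly MyCharacter, it casts player character 0 rather than that actor.
; If that character's Ammo is below the cap, it plays the CompileSuccess sound attached to its root, adds a fixed amount clamped to the cap, and destroys itself.
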(event OnComponentBeginOverlap(Box1)
  (params (OtherActor :type Actor%20Object%20Reference) (OtherComp :type Primitive%20Component%20Object%20Reference) (OtherBodyIndex :type Integer) (bFromSweep :type Boolean) (SweepResult :type Hit%20Result%20Structure%20%28by%20ref%29))
  (if (== (Utilities|GetClass OtherActor) "/Game/Blueprints/MyCharacter.MyCharacter_C")
    (bind _asmy_character (Utilities|Casting|CastToMyCharacter (Game|GetPlayerCharacter 0)))
    (if (< (Variables|/Game/Blueprints/MyCharacter.MyCharacter_C|GetAmmo _asmy_character) 100)
      (Class|GameplayStatics|PlaySoundAttached "/Engine/EditorSounds/Notifications/CompileSuccess.CompileSuccess" (VehicleSound|GetRootComponent) "None" "0, 0, 0" "EAttachLocation::KeepRelativeOffset")
      (Variables|/Game/Blueprints/MyCharacter.MyCharacter_C|SetAmmo _asmy_character (Math|Integer|Min(Integer) (+ (Variables|/Game/Blueprints/MyCharacter.MyCharacter_C|GetAmmo _asmy_character) 50) 100))
      (Actor|DestroyActor))))

(fn ConstructionScript)